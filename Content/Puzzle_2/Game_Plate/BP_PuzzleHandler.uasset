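; BP_PuzzleHandler runs an ordered light puzzle that opens BP_Door on completion.
; It finds BP_LightPuzzle actors and binds CheckCombination to the click event of those whose number matches the current step.
; CheckCombination either completes the puzzle at the final combination or advances the step and binds again.
; ResetPuzzle returns to the first step, rebinds and broadcasts lights out, with debug prints marking progress.
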(event Custom|IncrementCombination
  (bind _result (Math|Integer|IncrementInt (Variables|Default|GetCurrent%20Combination))
    (:%20%20
      (Development|PrintString (Utilities|String|ToString(Integer) _result))
      (CallFunction|BindtoLight))))

(event Custom|ResetPuzzle
  (Development|PrintString "Puzzle Reset")
  (Variables|Default|SetCurrent%20Combination 1)
  (CallFunction|BindtoLight)
  (Default|CallLightsOut))

(event Custom|BindToLight
  (bind _outactors (Actor|GetAllActorsOfClass "/Game/Puzzle_2/Game_Plate/BP_LightPuzzle.BP_LightPuzzle_C"))
  (for _array_element _outactors
    (if (== (Variables|/Game/Puzzle_2/Game_Plate/BP_LightPuzzle.BP_LightPuzzle_C|GetLightNumber _array_element) (Variables|Default|GetCurrent%20Combination))
      (EventDispatchers|BindEventtoClickInteraction _array_element (delegate Custom|CheckCombination)))))

(event Custom|CheckCombination
  (params (Light :type Integer))
  (if (== Light (Variables|Default|GetFinal%20Combination))
    (CallFunction|PuzzleComplete)
    (else
      (CallFunction|IncrementCombination))))

(event Custom|Puzzle%20Complete
  (bind _returnvalue (Actor|GetActorOfClass "/Game/Puzzle_2/Level_Design/BP_Door.BP_Door_C"))
  (Default|OpenDoor _returnvalue))

(event EventBeginPlay
  (CallFunction|BindtoLight)
  (Development|PrintString "Start Puzzle"))

(fn ConstructionScript)