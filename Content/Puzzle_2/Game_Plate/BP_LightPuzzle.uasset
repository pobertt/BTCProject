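; Interactable light for the light-order puzzle, checked against the combination held by BP_PuzzleHandler.
; On interact, it compares its LightNumber to the handler's CurrentCombination, then either calls CallClickInteraction and brightens its PointLight or resets the puzzle.
; It starts dimmed and binds to the handler's LightsOut event to dim again.
; OpenPuzzleWithDoor runs a timeline that moves PuzzleArrow along Z.
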(event Custom|OpenPuzzleWithDoor
  (bind _newtrack_0 (Timeline|Puzzle%20Open%20Timeline PlayFromStart)
    (:Update
      (Transformation|SetRelativeLocation (Variables|Default|GetPuzzleArrow) (Math|Vector|MakeVector 0.0 0.0 (Math|Float|Lerp (Variables|Default|GetRelative%20location) 2.5e+02 _newtrack_0)) false false))))

(event Custom|Interact
  (CallFunction|CheckCombination))

(event Custom|LightsOut
  (CallFunction|DimLight))

(event EventBeginPlay
  (CallFunction|DimLight)
  (bind _returnvalue (Actor|GetActorOfClass "/Game/Puzzle_2/Game_Plate/BP_PuzzleHandler.BP_PuzzleHandler_C"))
  (EventDispatchers|BindEventtoLightsOut _returnvalue (delegate Custom|LightsOut)))

(fn ConstructionScript)

(fn CheckCombination
  (bind _returnvalue (Actor|GetActorOfClass "/Game/Puzzle_2/Game_Plate/BP_PuzzleHandler.BP_PuzzleHandler_C"))
  (if (== (Variables|/Game/Puzzle_2/Game_Plate/BP_PuzzleHandler.BP_PuzzleHandler_C|GetCurrent%20Combination _returnvalue) (Variables|Default|GetLightNumber))
    (Default|CallClickInteraction (Variables|Default|GetLightNumber))
    (Rendering|Components|Light|SetIntensity (Variables|Default|GetPointLight) 1e+04)
    (else
      (Default|ResetPuzzle _returnvalue))))

(fn DimLight
  (Rendering|Components|Light|SetIntensity (Variables|Default|GetPointLight) 0.1))