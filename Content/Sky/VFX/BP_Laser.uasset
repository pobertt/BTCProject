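; BP_Laser is a Niagara laser beam actor that extends along its forward vector over time.
; Each Tick line-traces on the Camera channel, sets the beam end to the hit or trace end, then grows the trace distance up to a cap.
; An impact effect follows the hit point and shows only on a blocking hit.
; SetActive toggles only beam visibility, and the construction script tints both effects.
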(event Custom|Set%20Active
  (params (Input :type Boolean))
  (Rendering|SetVisibility (Variables|Default|GetNiagaraLaser) Input false))

(event EventBeginPlay)

(event Collision|EventActorBeginOverlap
  (params (OtherActor :type Actor%20Object%20Reference)))

(event EventTick
  (params (DeltaSeconds :type Float%20%28single-precision%29))
  (bind _returnvalue (Transformation|GetActorLocation))
  (Utilities|FlowControl|Sequence
    (:then_0
      (Variables|Default|SetTraceEnd (+ _returnvalue (* (Transformation|GetActorForwardVector) (Variables|Default|GetDistance))))
      (bind _outhit (Collision|LineTraceByChannel _returnvalue (+ _returnvalue (* (Transformation|GetActorForwardVector) (Variables|Default|GetDistance))) "TraceTypeQuery2" false 0 "None"))
      (Variables|Default|SetBlocking%20Hit (.bBlockingHit (Collision|BreakHitResult _outhit)))
      (Variables|Default|SetLocation (.Location (Collision|BreakHitResult _outhit)))
      (Effects|Components|ParticleSystem|SetVectorParameter (Variables|Default|GetNiagaraLaser) "BeamEnd" (Math|Vector|SelectVector (Variables|Default|GetLocation) (Variables|Default|GetTraceEnd) (Variables|Default|GetBlocking%20Hit)))
      (Rendering|SetVisibility (Variables|Default|GetNiagaraLaserEnd) (Variables|Default|GetBlocking%20Hit) false)
      (Transformation|SetWorldLocation (Variables|Default|GetNiagaraLaserEnd) (.Location (Collision|BreakHitResult _outhit)) false false))
    (:then_1
      (if (< (Variables|Default|GetDistance) 5e+04)
        (Variables|Default|SetDistance (+ (Variables|Default|GetDistance) (* DeltaSeconds 1.4e+03)))))))

(fn ConstructionScript
  (Effects|Components|ParticleSystem|SetColorParameter (Variables|Default|GetNiagaraLaser) "Colour" "(R=0.003241,G=0.006785,B=0.010000,A=1.000000)"))