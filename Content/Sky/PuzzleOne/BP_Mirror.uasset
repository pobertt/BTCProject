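; Possessable mirror for a light-beam puzzle, rotated with A/D (stand yaw) and W/S (clamped frame tilt), with E returning control to the player character.
; While Active, a looping timer line-traces the beam, activating any mirror struck on its glass or completing a BP_LightGoal once.
; When the beam misses, it deactivates the last hit mirror, and FUMirrorCheck switches off the one after that.
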(event Custom|LightUpdate
  (if (Variables|Default|GetActive?)
    (bind _outhit (Collision|LineTraceByChannel (Transformation|GetWorldLocation (Variables|Default|GetLightStart)) (Transformation|GetWorldLocation (Variables|Default|GetLightEnd)) "TraceTypeQuery1" false 0 "ForDuration" true "(R=1.000000,G=0.000000,B=0.000000,A=1.000000)" "(R=0.000000,G=1.000000,B=0.000000,A=1.000000)" 0.05))
    (bind _asbp_mirror (Utilities|Casting|CastToBP_Mirror (.HitActor (Collision|BreakHitResult _outhit)))
      (:then
        (Variables|Default|SetLast%20Hit%20Mirror _asbp_mirror)
        (if (== (Variables|BP_Mirror_C|GetMirror _asbp_mirror) (.HitComponent (Collision|BreakHitResult _outhit)))
          (Variables|BP_Mirror_C|SetActive? _asbp_mirror true)
          (else
            (Variables|BP_Mirror_C|SetActive? _asbp_mirror false)
            (Utilities|IsValid (Variables|Default|GetLast%20Hit%20Mirror)
              (:Is%20Valid
                (Variables|BP_Mirror_C|SetActive? (Variables|Default|GetLast%20Hit%20Mirror) false)
                ;[1 1 1] Repeat for as many mirrors as needed
                (CallFunction|FUMirrorCheck (Variables|Default|GetLast%20Hit%20Mirror)))))))
      (:CastFailed
        ;[1 1 1] sets last hit mirror to inactive
        (Utilities|FlowControl|Sequence
          (:then_0
            ;[1 1 1] create an end to the puzzle
            (bind _asbp_light_goal (Utilities|Casting|CastToBP_LightGoal (.HitActor (Collision|BreakHitResult _outhit))))
            (Utilities|FlowControl|DoOnce false
              (:Completed
                (Default|PuzzleComplete _asbp_light_goal))))
          (:then_1
            (Utilities|IsValid (Variables|Default|GetLast%20Hit%20Mirror)
              (:Is%20Valid
                (Variables|BP_Mirror_C|SetActive? (Variables|Default|GetLast%20Hit%20Mirror) false)
                ;[1 1 1] Repeat for as many mirrors as needed
                (CallFunction|FUMirrorCheck (Variables|Default|GetLast%20Hit%20Mirror))))))))))

(event Custom|Move%20Right
  (bind _stand (Variables|Default|GetStand))
  (bind _returnvalue (Transformation|GetRelativeTransform _stand))
  ;[1 1 1] Mirror Movement
  (Transformation|SetRelativeRotation _stand (Math|Rotator|MakeRotator (.roll (.rotation _returnvalue)) (.pitch (.rotation _returnvalue)) (+ (.yaw (.rotation _returnvalue)) (Variables|Default|GetHorizontal%20Sensitivity))) false false))

(event Custom|Move%20Left
  (bind _stand (Variables|Default|GetStand))
  (bind _returnvalue (Transformation|GetRelativeTransform _stand))
  ;[1 1 1] Mirror Movement
  (Transformation|SetRelativeRotation _stand (Math|Rotator|MakeRotator (.roll (.rotation _returnvalue)) (.pitch (.rotation _returnvalue)) (- (.yaw (.rotation _returnvalue)) (Variables|Default|GetHorizontal%20Sensitivity))) false false))

(event Custom|Move%20Up
  (bind _frame (Variables|Default|GetFrame))
  (bind _returnvalue (Transformation|GetRelativeTransform _frame))
  ;[1 1 1] Mirror Movement
  (Transformation|SetRelativeRotation _frame (Math|Rotator|MakeRotator (Math|Float|Clamp(Float) (- (.roll (.rotation _returnvalue)) (Variables|Default|GetVertical%20Sensitivity)) -4e+01 4e+01) (.pitch (.rotation _returnvalue)) (.yaw (.rotation _returnvalue))) false false))

(event Custom|Move%20Down
  (bind _frame (Variables|Default|GetFrame))
  (bind _returnvalue (Transformation|GetRelativeTransform _frame))
  ;[1 1 1] Mirror Movement
  (Transformation|SetRelativeRotation _frame (Math|Rotator|MakeRotator (Math|Float|Clamp(Float) (+ (.roll (.rotation _returnvalue)) (Variables|Default|GetVertical%20Sensitivity)) -4e+01 4e+01) (.pitch (.rotation _returnvalue)) (.yaw (.rotation _returnvalue))) false false))

(event EventBeginPlay
  (Utilities|Time|SetTimerbyEvent (delegate Custom|LightUpdate) 0.05 true)
  (Utilities|FlowControl|Delay 0.1)
  (Variables|Default|SetGame%20Started? true))

(event Collision|EventActorBeginOverlap
  (params (OtherActor :type Actor%20Object%20Reference)))

(event EventTick
  (params (DeltaSeconds :type Float%20%28single-precision%29)))

(event EventPossessed
  (params (NewController :type Controller%20Object%20Reference))
  ;[1 1 1] Character vis
  (if (Variables|Default|GetGame%20Started?)
    (Rendering|SetVisibility (Variables|Default|GetSkeletalMesh) true false)))

(event Input|KeyboardEvents|E
  (params (Key :type Key%20Structure :default "None"))
  ;[1 0 0] Robs code for interact here
  (:Pressed
    (bind _returnvalue (Actor|GetActorOfClass "/Game/Player/BP_PlayerCharacter.BP_PlayerCharacter_C"))
    (Rendering|SetVisibility (Variables|Default|GetSkeletalMesh) false false)
    (Pawn|Possess (Game|GetPlayerController 0) _returnvalue)))

(event Input|KeyboardEvents|W
  (params (Key :type Key%20Structure :default "None"))
  ;[1 1 1] Mirror Movement
  (:Pressed
    (bind _returnvalue (Utilities|Time|SetTimerbyEvent (delegate Custom|Move%20Up) 0.01 true)))
  (:Released
    (Utilities|Time|ClearandInvalidateTimerbyHandle _returnvalue)))

(event Input|KeyboardEvents|S
  (params (Key :type Key%20Structure :default "None"))
  ;[1 1 1] Mirror Movement
  (:Pressed
    (bind _returnvalue (Utilities|Time|SetTimerbyEvent (delegate Custom|Move%20Down) 0.01 true)))
  (:Released
    (Utilities|Time|ClearandInvalidateTimerbyHandle _returnvalue)))

(event Input|KeyboardEvents|D
  (params (Key :type Key%20Structure :default "None"))
  ;[1 1 1] Mirror Movement
  (:Pressed
    (bind _returnvalue (Utilities|Time|SetTimerbyEvent (delegate Custom|Move%20Right) 0.01 true)))
  (:Released
    (Utilities|Time|ClearandInvalidateTimerbyHandle _returnvalue)))

(event Input|KeyboardEvents|A
  (params (Key :type Key%20Structure :default "None"))
  ;[1 1 1] Mirror Movement
  (:Pressed
    (bind _returnvalue (Utilities|Time|SetTimerbyEvent (delegate Custom|Move%20Left) 0.01 true)))
  (:Released
    (Utilities|Time|ClearandInvalidateTimerbyHandle _returnvalue)))

(fn ConstructionScript)

(fn FUMirrorCheck
  (params (MirrortoCheck :type BP%20Mirror%20Object%20Reference))
  (bind _last_hit_mirror (Variables|BP_Mirror_C|GetLast%20Hit%20Mirror MirrortoCheck))
  (Utilities|IsValid _last_hit_mirror
    (:Is%20Valid
      (Variables|BP_Mirror_C|SetActive? _last_hit_mirror false)
      (return (Variables|BP_Mirror_C|GetLast%20Hit%20Mirror _last_hit_mirror)))))