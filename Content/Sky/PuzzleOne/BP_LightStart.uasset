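; BP_LightStart is the light source of a mirror puzzle, firing a repeating timer-driven visibility trace toward its LightEnd point, drawn as a debug line.
; It activates a BP_Mirror when the trace hits its Mirror component, and calls PuzzleComplete once on a directly hit BP_LightGoal.
; When the mirror component is missed, it deactivates the last hit mirror, and FUMirrorCheck deactivates the next mirror that one had hit.
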(event Custom|LightUpdate
  (bind _outhit (Collision|LineTraceByChannel (Transformation|GetWorldLocation (Variables|Default|GetDefaultSceneRoot)) (Transformation|GetWorldLocation (Variables|Default|GetLightEnd)) "TraceTypeQuery1" false 0 "ForDuration" true "(R=1.000000,G=0.000000,B=0.000000,A=1.000000)" "(R=0.000000,G=1.000000,B=0.000000,A=1.000000)" 0.05))
  (bind _asbp_mirror (Utilities|Casting|CastToBP_Mirror (.HitActor (Collision|BreakHitResult _outhit)))
    (:then
      (Variables|Default|SetLast%20Hit%20Mirror _asbp_mirror)
      (if (== (Variables|/Game/Sky/PuzzleOne/BP_Mirror.BP_Mirror_C|GetMirror _asbp_mirror) (.HitComponent (Collision|BreakHitResult _outhit)))
        (Variables|/Game/Sky/PuzzleOne/BP_Mirror.BP_Mirror_C|SetActive? _asbp_mirror true)
        (else
          (Variables|/Game/Sky/PuzzleOne/BP_Mirror.BP_Mirror_C|SetActive? _asbp_mirror false)
          (Utilities|IsValid (Variables|Default|GetLast%20Hit%20Mirror)
            (:Is%20Valid
              (Variables|/Game/Sky/PuzzleOne/BP_Mirror.BP_Mirror_C|SetActive? (Variables|Default|GetLast%20Hit%20Mirror) false)
              ;[1 1 1] Repeat for as many mirrors as needed
              (CallFunction|FUMirrorCheck (Variables|Default|GetLast%20Hit%20Mirror)))))))
    (:CastFailed
      ;[1 1 1] sets last hit mirror to inactive
      (Utilities|FlowControl|Sequence
        (:then_0
          ;[1 1 1] create an end to the puzzle
          (bind _asbp_light_goal (Utilities|Casting|CastToBP_LightGoal (.HitActor (Collision|BreakHitResult _outhit))))
          (Utilities|FlowControl|DoOnce false
            (:Completed
              (Default|PuzzleComplete _asbp_light_goal))))
        (:then_1
          (Utilities|IsValid (Variables|Default|GetLast%20Hit%20Mirror)
            (:Is%20Valid
              (Variables|/Game/Sky/PuzzleOne/BP_Mirror.BP_Mirror_C|SetActive? (Variables|Default|GetLast%20Hit%20Mirror) false)
              ;[1 1 1] Repeat for as many mirrors as needed
              (CallFunction|FUMirrorCheck (Variables|Default|GetLast%20Hit%20Mirror)))))))))

(event EventBeginPlay
  (Utilities|Time|SetTimerbyEvent (delegate Custom|LightUpdate) 0.05 true))

(event Collision|EventActorBeginOverlap
  (params (OtherActor :type Actor%20Object%20Reference)))

(event EventTick
  (params (DeltaSeconds :type Float%20%28single-precision%29)))

(fn ConstructionScript)

(fn FUMirrorCheck
  (params (MirrortoCheck :type BP%20Mirror%20Object%20Reference))
  (bind _last_hit_mirror (Variables|/Game/Sky/PuzzleOne/BP_Mirror.BP_Mirror_C|GetLast%20Hit%20Mirror MirrortoCheck))
  (Utilities|IsValid _last_hit_mirror
    (:Is%20Valid
      (Variables|/Game/Sky/PuzzleOne/BP_Mirror.BP_Mirror_C|SetActive? _last_hit_mirror false)
      (return (Variables|/Game/Sky/PuzzleOne/BP_Mirror.BP_Mirror_C|GetLast%20Hit%20Mirror _last_hit_mirror)))))