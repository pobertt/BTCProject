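; BP_LeonPlayerCharacter is the player character, handling input setup, the pause menu, colour vision settings and switching control to mirrors.
; The pause action toggles W_PauseMenu, game pause, input mode and cursor, while UpdateColourBlindness applies the selected vision deficiency type.
; Pressing E hides the mesh and possesses the nearest BP_Mirror with no range check; being possessed again shows the mesh.
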(event Custom|UpdateColourBlindness
  ;[1 1 1] Colour Blindness
  (switch int (Variables|Default|GetColourBlindness)
    (:0
      (Variables|Default|SetType "NormalVision"))
    (:1
      (Variables|Default|SetType "Deuteranope"))
    (:2
      (Variables|Default|SetType "Protanope"))
    (:3
      (Variables|Default|SetType "Tritanope")))
  (Class|WidgetBlueprintLibrary|SetColorVisionDeficiencyType (Variables|Default|GetType) (Variables|Default|GetSeverity) (Variables|Default|GetCorrect%20Deficiency)))

(event Input|EnhancedActionEvents|EnhancedInputActionIA_PauseGame
  (params (ActionValue :type Boolean) (ElapsedSeconds :type Float%20%28double-precision%29) (TriggeredSeconds :type Float%20%28double-precision%29) (InputAction :type Input%20Action%20Object%20Reference :default "/Game/ThirdPerson/Input/Actions/IA_PauseGame.IA_PauseGame"))
  (bind _returnvalue (Game|GetPlayerController 0))
  ;[1 1 1] Pause Game
  (:Started
    (if (not (Variables|Default|GetIsPauseMenuOpened?))
      (Variables|Default|SetIsPauseMenuOpened? true)
      (bind _returnvalue_2 (UserInterface|CreateWidget "/Game/Widget/W_PauseMenu.W_PauseMenu_C" _returnvalue))
      (bind _output_get (Variables|Default|SetPause%20Menu%20Widget _returnvalue_2))
      (UserInterface|Viewport|AddtoViewport _output_get 0)
      (Input|SetInputModeGameandUI _returnvalue (Variables|Default|GetPause%20Menu%20Widget) "DoNotLock" true false)
      (Variables|/Script/Engine.PlayerController|SetbShowMouseCursor (Game|GetPlayerController 0) true)
      (Game|SetGamePaused true)
      (else
        (Variables|Default|SetIsPauseMenuOpened? false)
        (Widget|RemovefromParent (Variables|Default|GetPause%20Menu%20Widget))
        (Game|SetGamePaused false)
        (Input|SetInputModeGameOnly _returnvalue false)
        (Variables|/Script/Engine.PlayerController|SetbShowMouseCursor (Game|GetPlayerController 0) false)))))

(event EventPossessed
  (params (NewController :type Controller%20Object%20Reference))
  ;[1 1 1] Character vis on interact
  (Rendering|SetVisibility (Variables|Character|GetMesh) true false))

(event Collision|EventActorBeginOverlap
  (params (OtherActor :type Actor%20Object%20Reference)))

(event EventBeginPlay
  (bind _returnvalue (Game|GetPlayerController 0))
  (Input|AddMappingContext (PlayerController|LocalPlayerSubsystems|GetEnhancedInputLocalPlayerSubsystem _returnvalue) "/Game/Player/Input/MainMappingContext.MainMappingContext" 0 "(bIgnoreAllPressedKeysUntilRelease=True,bForceImmediately=False)")
  (Input|SetInputModeGameOnly _returnvalue false))

(event Input|KeyboardEvents|E
  (params (Key :type Key%20Structure :default "None"))
  ;[1 0 0] Robs code for interact here
  (:Pressed
    (bind _outactors (Actor|GetAllActorsOfClass "/Game/Sky/PuzzleOne/BP_Mirror.BP_Mirror_C"))
    (bind _asbp_mirror (Utilities|Casting|CastToBP_Mirror (.ReturnValue (Actor|FindNearestActor (Transformation|GetActorLocation) _outactors))))
    (Rendering|SetVisibility (Variables|Character|GetMesh) false false)
    (Pawn|Possess (Game|GetPlayerController 0) _asbp_mirror)))

(fn ConstructionScript)