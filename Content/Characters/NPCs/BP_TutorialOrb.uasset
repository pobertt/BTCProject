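; Tutorial orb NPC that shows a multi-line dialogue box when the player presses E inside its overlap box.
; Tick polls for E during overlap, creates the WBP_DialogueBox widget on first press and calls ArrayLooperDialogue.
; That function steps text and sprite arrays by a shared index, then removes the widget and resets past the end.
; A separate E key event also advances the dialogue without checking overlap.
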(event OnComponentBeginOverlap(Box)
  (params (OverlappedComponent :type Primitive%20Component%20Object%20Reference) (OtherActor :type Actor%20Object%20Reference) (OtherComp :type Primitive%20Component%20Object%20Reference) (OtherBodyIndex :type Integer) (bFromSweep :type Boolean) (SweepResult :type Hit%20Result%20Structure%20%28by%20ref%29))
  (Variables|Default|SetisOverlapping true))

(event OnComponentEndOverlap(Box)
  (params (OverlappedComponent :type Primitive%20Component%20Object%20Reference) (OtherActor :type Actor%20Object%20Reference) (OtherComp :type Primitive%20Component%20Object%20Reference) (OtherBodyIndex :type Integer))
  (Variables|Default|SetisOverlapping false))

(event EventBeginPlay
  (Variables|Default|SetDisplayedText (Utilities|Array|Get(acopy) (Variables|Default|GetDialogueArrayOrb) (Variables|Default|GetCurrentArrayIndex))))

(event Collision|EventActorBeginOverlap
  (params (OtherActor :type Actor%20Object%20Reference)))

(event EventTick
  (params (DeltaSeconds :type Float%20%28single-precision%29))
  (Utilities|Time|SetTimerbyEvent 0 DeltaSeconds true)
  (if (Variables|Default|GetisOverlapping)
    (if (Game|Player|WasInputKeyJustPressed (Game|GetPlayerController 0) "E")
      (if (Variables|Default|GetisDialogueHappening)
        _
        (else
          (CallFunction|OpenWidget)
          (bind _output_get (Variables|Default|SetisDialogueHappening true))))
      (if _output_get
        (if (Game|Player|WasInputKeyJustPressed (Game|GetPlayerController 0) "E")
          (CallFunction|ArrayLooperDialogue))))))

(event Input|KeyboardEvents|E
  (params (Key :type Key%20Structure :default "None"))
  (:Pressed
    (if (Game|Player|WasInputKeyJustPressed (Game|GetPlayerController 0) "E")
      (CallFunction|ArrayLooperDialogue))))

(fn ConstructionScript)

(fn OpenWidget
  (bind _returnvalue (UserInterface|CreateWidget "/Game/UIandWidgets/Widgets/WBP_DialogueBox.WBP_DialogueBox_C" (Game|GetPlayerController 0)))
  (Variables|Default|SetCurrentWidget _returnvalue)
  (UserInterface|Viewport|AddtoViewport _returnvalue 0)
  (Appearance|SetBrushfromTexture (Variables|/Game/UIandWidgets/Widgets/WBP_DialogueBox.WBP_DialogueBox_C|GetPopupSprite _returnvalue) "/SpeedTreeImporter/SpeedTree9/Empty.Empty" true))

(fn ArrayLooperDialogue
  (CallFunction|ArrayLooperSprites)
  (Variables|Default|SetDisplayedText (Utilities|Array|Get(acopy) (Variables|Default|GetDialogueArrayOrb) (Variables|Default|GetCurrentArrayIndex)))
  (if (< (Variables|Default|GetCurrentArrayIndex) (Utilities|Array|Length (Variables|Default|GetDialogueArrayOrb)))
    (Variables|Default|SetCurrentArrayIndex (+ (Variables|Default|GetCurrentArrayIndex) 1))
    (else
      (Class|GameViewportSubsystem|RemoveWidget (|GameViewportSubsystem) (Variables|Default|GetCurrentWidget))
      (Variables|Default|SetisDialogueHappening false)
      (Variables|Default|SetCurrentArrayIndex 0))))

(fn ArrayLooperSprites
  (Variables|Default|SetCurrentSpriteSB (Class|PaperSpriteBlueprintLibrary|MakeBrushfromSprite (Utilities|Array|Get(acopy) (Variables|Default|GetSprite%20Array) (Variables|Default|GetCurrentArrayIndex)) 1 1)))