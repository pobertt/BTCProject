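; Player controller that toggles possession between a Game_Plate actor and the CAM_PlayerCharacter when F is pressed.
; A FlipFlop alternates the target, finding the first actor of each class with GetAllActorsOfClass and possessing it.
; The mouse cursor shows while possessing the plate and hides when control returns to the character.
; An unused Posses function is empty, and a disconnected copy of the plate branch remains.
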(event Input|KeyboardEvents|F
  (params (Key :type Key%20Structure :default "None"))
  (:Pressed
    (Utilities|FlowControl|FlipFlop
      (:A
        (bind _outactors (Actor|GetAllActorsOfClass "/Game/Puzzle_2/Game_Plate/Game_Plate.Game_Plate_C"))
        (Pawn|Possess (Utilities|Array|Get(acopy) _outactors))
        (Variables|Default|SetbShowMouseCursor true))
      (:B
        (bind _outactors_2 (Actor|GetAllActorsOfClass "/Game/Player/CAM_PlayerCharacter.CAM_PlayerCharacter_C"))
        (Pawn|Possess (Utilities|Array|Get(acopy) _outactors_2))
        (Variables|Default|SetbShowMouseCursor false)))))

(fn ConstructionScript)

(fn Posses)